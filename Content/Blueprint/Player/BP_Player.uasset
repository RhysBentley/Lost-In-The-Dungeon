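; Player character that moves along one axis, with mesh turning, walking, jumping, an inventory and a four-slot item select wheel.
; Input events toggle HUD widgets and cursor mode, while wheel picks fill the main or off hand by slot type.
; Timed animations with a movement lock handle melee attacks and moving the weapon between back and hand sockets.
; Off-hand items are used through a briefly spawned actor, and drops refresh inventory, wheel and hand slots.
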(event `self.ReceiveBeginPlay`
  ;[0 0 0] Creates the HUD Widget
  (bind _returnvalue (`|CreateWidget` "/Game/Widgets/Widget_HUD.Widget_HUD_C"))
  (bind _output_get (set `self.HUDReference` _returnvalue))
  (`UserWidget.AddToViewport` _output_get 0))

(event `InputAxis|Walk`
  (params (AxisValue :type "Float (single-precision)"))
  ;[0 0 0] Movement
  ;;[0 0 0] Basic Movement
  (if (not (or (`NavMovementComponent.IsFalling` (`self.CharacterMovement`)) (`self.CantMove`)))
    (`self.AddMovementInput` (0.0 1.0 0.0) AxisValue)
    (`/Engine/EditorBlueprintResources/StandardMacros.CompareFloat` AxisValue ; Rotates Mesh Left and Right
      (:`>`
        (bind (_direction _alpha) (`Timeline|RotatingMesh` :!via `Reverse` :!label _label)
          (:`Update`
            (`SceneComponent.K2_SetRelativeRotation` (`self.Mesh`) (`KismetMathLibrary.RLerp` (struct :`Yaw` -90.0) (struct :`Yaw` -270.0) _alpha) false false))))
      (:`<`
        (goto _label)))))

(event `InputAction|Walking`
  (params (Key :type "Key Structure"))
  (bind _charactermovement (`self.CharacterMovement`))
  ;[0 0 0] Movement
  ;;[0 0 0] Sprinting
  (:`Pressed`
    (set `CharacterMovementComponent.MaxWalkSpeed` 200.0 _charactermovement))
  (:`Released`
    (set `CharacterMovementComponent.MaxWalkSpeed` 600.0 _charactermovement)))

(event `InputAction|Jump`
  (params (Key :type "Key Structure"))
  ;[0 0 0] Movement
  ;;[0 0 0] Jumping
  (:`Pressed`
    (`self.Jump`))
  (:`Released`
    (`self.StopJumping`)))

(event `InputAction|Inventory`
  (params (Key :type "Key Structure"))
  (bind _widget_inventory (`/Game/Widgets/Widget_HUD.Widget_Inventory` (`self.HUDReference`)))
  ;[0 0 0] Opens/Closes the inventory
  (:`Pressed`
    (`/Engine/EditorBlueprintResources/StandardMacros.FlipFlop`
      (:`A`
        (`Widget.SetVisibility` _widget_inventory "Visible")
        (`self.ChangeCursorState` true))
      (:`B`
        (`Widget.SetVisibility` _widget_inventory "Hidden")
        (`/Game/Widgets/Widget_HUD.HideToolTips` (`self.HUDReference`))
        (`self.ChangeCursorState` false)))))

(event `InputAction|SelectWheel`
  (params (Key :type "Key Structure"))
  (bind _widget_selectwheel (`/Game/Widgets/Widget_HUD.Widget_SelectWheel` (`self.HUDReference`)))
  (bind _widget_selectwheel_2 (`/Game/Widgets/Widget_HUD.Widget_SelectWheel` (`self.HUDReference`)))
  ;[0 0 0] Opens/Closes the Select Wheel
  (:`Pressed`
    (`Widget.SetVisibility` _widget_selectwheel_2 "Visible")
    (`/Game/Widgets/Widget_SelectWheel.EnableSelectWheelSlot` _widget_selectwheel_2)
    (`self.ChangeCursorState` true))
  (:`Released`
    (`Widget.SetVisibility` _widget_selectwheel "Hidden")
    (switch `/Game/Enumeration/Enum_SelectWheel` (`/Game/Widgets/Widget_SelectWheel.SelectedArea` _widget_selectwheel)
      (:`NewEnumerator0`
        (`self.SettingItem` (`.TopLeft_2_D25FFC834CE706FB57033793BC9C5387` (break `/Game/Structure/Struct_SelectWheelItems` (`self.SelectWheelItems`)))))
      (:`NewEnumerator1`
        (`self.SettingItem` (`.TopRight_6_3DF5F0024799EDFEB19DC3836F372DF9` (break `/Game/Structure/Struct_SelectWheelItems` (`self.SelectWheelItems`)))))
      (:`NewEnumerator2`
        (`self.SettingItem` (`.BottomLeft_7_85C2A3884310FACBE49B878E34226B3A` (break `/Game/Structure/Struct_SelectWheelItems` (`self.SelectWheelItems`)))))
      (:`NewEnumerator3`
        (`self.SettingItem` (`.BottomRight_8_20731D2F45F6019A61FE9882AA8FBC3B` (break `/Game/Structure/Struct_SelectWheelItems` (`self.SelectWheelItems`))))))
    (`self.ChangeCursorState` false)))

(event `InputAction|Equip/Unequip`
  (params (Key :type "Key Structure"))
  (bind _mesh (`self.Mesh`))
  (bind _mainhandmesh (`self.MainHandMesh`))
  (bind _mesh_2 (`self.Mesh`))
  (bind _mainhandmesh_2 (`self.MainHandMesh`))
  ;[0 0 0] Equiping and Unequiping the Weapon
  (:`Pressed`
    (if (`KismetSystemLibrary.IsValidClass` (`.BlueprintClass_12_A3BE8845484EA4E75981A09D99305B41` (break `/Game/Structure/Struct_InventoryItem` (`self.MainHand`))))
      (if (not (`self.IsArmed`))
        ;;[0 0 0] Equiping the Weapon to the Hand
        (set `self.CantMove` true)
        (`SkeletalMeshComponent.PlayAnimation` _mesh_2 "/Game/Animations/Player/Unarmed/Unarmed_Equip_Over_Shoulder.Unarmed_Equip_Over_Shoulder" false)
        (`KismetSystemLibrary.Delay` 0.4)
        (`SceneComponent.K2_DetachFromComponent` _mainhandmesh_2 "KeepWorld" "KeepWorld" "KeepWorld" true)
        (`SceneComponent.K2_AttachToComponent` _mainhandmesh_2 _mesh_2 "RightHandSocket" "SnapToTarget" "SnapToTarget" "SnapToTarget" true)
        (`KismetSystemLibrary.Delay` 0.435)
        (`SkeletalMeshComponent.SetAnimationMode` _mesh_2 "AnimationBlueprint")
        (set `self.IsArmed` true)
        (set `self.CantMove` false)
        (else
          ;;[0 0 0] Unequiping the Weapon from the Hand
          (set `self.CantMove` true)
          (`SkeletalMeshComponent.PlayAnimation` _mesh "/Game/Animations/Player/Armed/Standing_Disarm_Over_Shoulder.Standing_Disarm_Over_Shoulder" false)
          (`KismetSystemLibrary.Delay` 0.4)
          (`SceneComponent.K2_DetachFromComponent` _mainhandmesh "KeepWorld" "KeepWorld" "KeepWorld" true)
          (`SceneComponent.K2_AttachToComponent` _mainhandmesh _mesh "WeaponSocket" "SnapToTarget" "SnapToTarget" "SnapToTarget" true)
          (`KismetSystemLibrary.Delay` 0.435)
          (`SkeletalMeshComponent.SetAnimationMode` _mesh "AnimationBlueprint")
          (set `self.IsArmed` false)
          (set `self.CantMove` false))))))

(event `DropItem`
  (params (ItemInfo :type "/Game/Structure/Struct_InventoryItem Structure"))
  ;[0 0 0] Drops an item
  (`/Game/Blueprint/Inventory/BP_InventoryComponent.DropItem` (`self.BP_InventoryComponent`) ItemInfo (`SceneComponent.K2_GetComponentToWorld` (`self.ItemSpawn`)))
  (`/Game/Widgets/Inventory/Widget_Inventory.UpdateInventorySlots` (`/Game/Widgets/Widget_HUD.Widget_Inventory` (`self.HUDReference`)))
  (`self.SetSelectWheelSlot` (`self.MainHand`))
  (`self.SetSelectWheelSlot` (`self.OffHand`))
  (`self.SettingSlots` ItemInfo))

(event `InputAction|MainHand`
  (params (Key :type "Key Structure"))
  (bind _mesh (`self.Mesh`))
  ;[0 0 0] Pressing Main Hand Button
  (:`Pressed`
    (if (and (`self.IsArmed`) (not (`self.CantMove`)))
      (set `self.CantMove` true)
      (`SkeletalMeshComponent.PlayAnimation` _mesh "/Game/Animations/Player/Armed/Attacks/Standing_Melee_Attack_Horizontal.Standing_Melee_Attack_Horizontal" false)
      (`KismetSystemLibrary.Delay` 2.4)
      (`SkeletalMeshComponent.SetAnimationMode` _mesh "AnimationBlueprint")
      (set `self.CantMove` false))))

(event `InputAction|OffHand`
  (params (Key :type "Key Structure"))
  (bind _offhand (`self.OffHand`))
  (bind ((`ID_27_F5629E724BE2FB4174B3D4B082B40F19` _id) (`BlueprintClass_12_A3BE8845484EA4E75981A09D99305B41` _blueprintclass)) (break `/Game/Structure/Struct_InventoryItem` _offhand))
  ;[0 0 0] Pressing Off Hand Button
  (:`Pressed`
    (if (`KismetSystemLibrary.IsValidClass` (`.BlueprintClass_12_A3BE8845484EA4E75981A09D99305B41` (break `/Game/Structure/Struct_InventoryItem` (`self.OffHand`))))
      (bind _returnvalue (`|SpawnActorFromClass` _blueprintclass (`KismetMathLibrary.MakeTransform` (0.0 0.0 0.0) (struct) (0.0 0.0 0.0)) "Undefined" "OverrideRootScale" null _offhand _id null))
      (`/Game/Blueprint/Inventory/Items/BP_Item__Master.UseItem` _returnvalue)
      (`self.K2_DestroyActor` _returnvalue))))

(fn `ChangeCursorState`
  (params (Enable :type Boolean))
  (bind _returnvalue (`GameplayStatics.GetPlayerController` 0))
  (if Enable
    (set `PlayerController.bShowMouseCursor` true _returnvalue)
    (`WidgetBlueprintLibrary.SetInputMode_GameAndUIEx` _returnvalue (`self.HUDReference`))
    (return)
    (else
      (set `PlayerController.bShowMouseCursor` false _returnvalue)
      (`WidgetBlueprintLibrary.SetInputMode_GameOnly` _returnvalue)
      (return))))

(fn `CheckHeightFromGround`
  (returns (Distance :type "Float (double-precision)"))
  (bind _mesh (`self.Mesh`))
  (bind _returnvalue (`SceneComponent.K2_GetComponentLocation` _mesh))
  (bind _outhit (`KismetSystemLibrary.LineTraceSingleForObjects` _returnvalue (+ _returnvalue (* (* (`SceneComponent.GetUpVector` _mesh) 200.0) -1.0)) (`|MakeArray` "ObjectTypeQuery1" :!type "EObjectTypeQuery Enum")))
  (return (`KismetMathLibrary.Vector_Distance` (`SceneComponent.K2_GetComponentLocation` (`self.Mesh`)) (`.Location` (`GameplayStatics.BreakHitResult` _outhit)))))

(fn `EqualItemStructures`
  (params (Find :type "/Game/Structure/Struct_InventoryItem Structure") (LookThrough :type "/Game/Structure/Struct_InventoryItem Structure"))
  (returns (IsStruct :type Boolean))
  (return (== (`.BlueprintClass_12_A3BE8845484EA4E75981A09D99305B41` (break `/Game/Structure/Struct_InventoryItem` Find)) (`.BlueprintClass_12_A3BE8845484EA4E75981A09D99305B41` (break `/Game/Structure/Struct_InventoryItem` LookThrough)))))

(fn `SetSelectWheelSlot`
  (params (FindStruct :type "/Game/Structure/Struct_InventoryItem Structure"))
  (bind (_topleft _topright _bottomleft _bottomright) (break `/Game/Structure/Struct_SelectWheelItems` (`self.SelectWheelItems`)))
  (bind _widget_selectwheel (`/Game/Widgets/Widget_HUD.Widget_SelectWheel` (`self.HUDReference`)))
  (if (`self.EqualItemStructures` FindStruct _topleft)
    (`/Game/Widgets/Widget_SelectWheel.SettingInfo` :`self` _widget_selectwheel)
    (elif (`self.EqualItemStructures` FindStruct _topright)
      (`/Game/Widgets/Widget_SelectWheel.SettingInfo` :`self` _widget_selectwheel :`AreaToChange` "NewEnumerator1")
      (elif (`self.EqualItemStructures` FindStruct _bottomleft)
        (`/Game/Widgets/Widget_SelectWheel.SettingInfo` :`self` _widget_selectwheel :`AreaToChange` "NewEnumerator2")
        (elif (`self.EqualItemStructures` FindStruct _bottomright)
          (`/Game/Widgets/Widget_SelectWheel.SettingInfo` :`self` _widget_selectwheel :`AreaToChange` "NewEnumerator3")))))
  (return))

(fn `SettingItem`
  (params (ItemInfo :type "/Game/Structure/Struct_InventoryItem Structure (by ref)"))
  (bind _mainhandmesh (`self.MainHandMesh`))
  (if (`|EnumEquality` (`.SlotType_30_4D430619487C58BF940A7D977B79608E` (break `/Game/Structure/Struct_InventoryItem` ItemInfo)) "NewEnumerator0")
    (bind _output_get (set `self.MainHand` ItemInfo))
    (`StaticMeshComponent.SetStaticMesh` _mainhandmesh (`.StaticMesh_8_0B6818A94C13B8EBCB6B1B892388F204` (break `/Game/Structure/Struct_InventoryItem` _output_get)))
    (`SceneComponent.SetVisibility` _mainhandmesh true false)
    (else
      (set `self.OffHand` ItemInfo)))
  (`/Game/Widgets/Widget_Slot.UpdateSlotsInfo` (`/Game/Widgets/Widget_HUD.Widget_Slot` (`self.HUDReference`))))

(fn `SettingSlots`
  (params (`Dropped/UsedItem` :type "/Game/Structure/Struct_InventoryItem Structure (by ref)"))
  (locals (Temp_Item :type "/Game/Structure/Struct_InventoryItem Structure"))
  (bind ((`BlueprintClass_12_A3BE8845484EA4E75981A09D99305B41` _blueprintclass)) (break `/Game/Structure/Struct_InventoryItem` `Dropped/UsedItem`))
  (bind _temp_item (`local.Temp_Item`))
  (set `local.Temp_Item` `Dropped/UsedItem`)
  (if (== _blueprintclass (`.BlueprintClass_12_A3BE8845484EA4E75981A09D99305B41` (break `/Game/Structure/Struct_InventoryItem` (`self.MainHand`))))
    (set `self.MainHand` (struct))
    (`/Game/Widgets/Widget_Slot.UpdateSlotsInfo` (`/Game/Widgets/Widget_HUD.Widget_Slot` (`self.HUDReference`)))
    (elif (== _blueprintclass (`.BlueprintClass_12_A3BE8845484EA4E75981A09D99305B41` (break `/Game/Structure/Struct_InventoryItem` (`self.OffHand`))))
      (if (<= (`.Quantity_25_CCABC0304EA3051D0B5A609EAA090952` (break `/Game/Structure/Struct_InventoryItem` (`local.Temp_Item`))) 1)
        (set `self.OffHand` (struct))
        (`/Game/Widgets/Widget_Slot.UpdateSlotsInfo` (`/Game/Widgets/Widget_HUD.Widget_Slot` (`self.HUDReference`)))
        (else
          (bind _structout (setmembers `/Game/Structure/Struct_InventoryItem` :`StructRef` _temp_item :`Quantity` (- (`.Quantity_25_CCABC0304EA3051D0B5A609EAA090952` (break `/Game/Structure/Struct_InventoryItem` _temp_item)) 1)))
          (`self.SettingItem` _structout))))))

(fn `UserConstructionScript`)