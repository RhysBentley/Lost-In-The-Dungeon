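; BP_Enemy is a melee enemy character that senses the player, attacks with a weapon and ragdolls on death.
; Sight and CanAttack overlaps set blackboard keys on its AI controller, while BPStatsComponent handles damage and feeds a health bar turned toward the player's camera.
; Attacks and hit reactions temporarily override the AnimBP, with DoOnce gates limiting weapon hits.
; Death swaps the mesh for an impulse-driven ragdoll, then destroys the actor.
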(event `self.ReceiveBeginPlay`
  (bind _bp_statscomponent (`self.BP_StatsComponent`))
  ;[1 1 1] Event BeginPlay
  ;;[1 1 1] Getting Reference
  (bind _asbp_player (cast `/Game/Blueprint/Player/BP_Player` (`GameplayStatics.GetPlayerCharacter` 0)))
  (set `self.PlayerReference` _asbp_player)
  (bind _aswidget_enemy_stats (cast `/Game/Widgets/Widget_EnemyStats` (`WidgetComponent.GetUserWidgetObject` (`self.HealthBar`))))
  (set `self.HealthBarReference` _aswidget_enemy_stats)
  (bind _asbp_enemy_controller (cast `/Game/Blueprint/Enemy/Controllers/BP_EnemyController` (`self.GetController`)))
  (set `self.ControllerReference` _asbp_enemy_controller)
  ;;[1 1 1] Update the Widget
  (`/Game/Widgets/Widget_EnemyStats.UpdateWidget` (`self.HealthBarReference`) (`/Game/Blueprint/BP_StatsComponent.Health` _bp_statscomponent) (`/Game/Blueprint/BP_StatsComponent.MaxHealth` _bp_statscomponent)))

(event `RotateMesh`
  ;[1 1 1] Rotating the Mesh when turning around
  (bind (_direction _alpha) (`Timeline|RotateMeshTimeline` :!via `PlayFromStart`)
    (:`Update`
      (`SceneComponent.K2_SetRelativeRotation` (`self.Mesh`) (`KismetMathLibrary.RLerp` (struct :`Yaw` -90.0) (struct :`Yaw` -270.0) _alpha) false false))
    (:`Finished`
      (`KismetSystemLibrary.Delay` 0.05) ; Used to remove small glitch
      (`SceneComponent.K2_SetRelativeRotation` (`self.Mesh`) (struct :`Yaw` -90.0) false false))))

(event `self.ReceiveTick`
  (params (DeltaSeconds :type "Float (single-precision)"))
  ;[1 1 1] Rotating the Health Bar
  (if (not (or (`self.IsDead`) (`self.IsPlayerDead`)))
    (`SceneComponent.K2_SetWorldRotation` (`self.HealthBar`) (`KismetMathLibrary.FindLookAtRotation` (`SceneComponent.K2_GetComponentLocation` (`self.HealthBar`)) (`SceneComponent.K2_GetComponentLocation` (`/Game/Blueprint/Player/BP_Player.Camera` (`self.PlayerReference`)))) false false)
    (`self.Test` DeltaSeconds)))

(event `self.ReceiveAnyDamage`
  (params (Damage :type "Float (single-precision)") (DamageType :type "DamageType Object Reference") (InstigatedBy :type "Controller Object Reference") (DamageCauser :type "Actor Object Reference"))
  (bind _blood (`self.Blood`))
  (bind _bp_statscomponent (`self.BP_StatsComponent`))
  ;[1 1 1] Taking Damage
  (bind _hasdied (`/Game/Blueprint/BP_StatsComponent.Take Damage` (`self.BP_StatsComponent`) (`KismetMathLibrary.FTrunc` Damage)))
  (`/Game/Widgets/Widget_EnemyStats.UpdateWidget` (`self.HealthBarReference`) (`/Game/Blueprint/BP_StatsComponent.Health` _bp_statscomponent) (`/Game/Blueprint/BP_StatsComponent.MaxHealth` _bp_statscomponent))
  (if _hasdied
    (`ActorComponent.Activate` _blood false)
    (`self.Death`)
    (else
      (`ActorComponent.Activate` _blood false)
      (`self.InterruptAttack`)
      (`SkeletalMeshComponent.PlayAnimation` (`self.Mesh`) "/Game/Animations/Enemy/Standing_React_Large_From_Left.Standing_React_Large_From_Left" false)
      (`KismetSystemLibrary.Delay` 1.03)
      (`SkeletalMeshComponent.SetAnimationMode` (`self.Mesh`) "AnimationBlueprint"))))

(event `Death`
  ;[1 1 1] Death Event
  (set `self.IsDead` true)
  (`ActorComponent.K2_DestroyComponent` (`self.Mesh`))
  (`ActorComponent.K2_DestroyComponent` (`self.HealthBar`))
  (`ActorComponent.K2_DestroyComponent` (`self.CapsuleComponent`))
  (`SceneComponent.SetVisibility` (`self.Ragdoll`) true false)
  (`PrimitiveComponent.SetSimulatePhysics` (`self.Weapon`) true)
  (`PrimitiveComponent.SetSimulatePhysics` (`self.Ragdoll`) true)
  (`SkeletalMeshComponent.AddImpulseToAllBodiesBelow` (`self.Ragdoll`) (select `bool` (<= (`self.GetDotProductTo` (`self.PlayerReference`) self) 0.0) :`false` (0.0 -600.0 0.0) :`true` (0.0 600.0 0.0) :!type "Vector Structure") "spine_03" false true)
  (`KismetSystemLibrary.Delay` 3.0)
  (`self.K2_DestroyActor`))

(event `self.Sight.OnComponentBeginOverlap`
  (params (OverlappedComponent :type "PrimitiveComponent Object Reference") (OtherActor :type "Actor Object Reference") (OtherComp :type "PrimitiveComponent Object Reference") (OtherBodyIndex :type Integer) (bFromSweep :type Boolean) (SweepResult :type "HitResult Structure (by ref)"))
  ;[1 1 1] Attacking the Player
  ;;[1 1 1] Detecting if the Enemy can see the player
  (cast `/Game/Blueprint/Player/BP_Player` OtherActor)
  (if (not (`self.IsDead`))
    (set `self.CanSee` true)
    (`BlackboardComponent.SetValueAsBool` (`/Game/Blueprint/Enemy/Controllers/BP_EnemyController.Blackboard Component` (`self.ControllerReference`)) "CanSee" true)
    (`BlackboardComponent.SetValueAsObject` (`/Game/Blueprint/Enemy/Controllers/BP_EnemyController.Blackboard Component` (`self.ControllerReference`)) "PlayerReference" (`self.PlayerReference`))))

(event `self.Sight.OnComponentEndOverlap`
  (params (OverlappedComponent :type "PrimitiveComponent Object Reference") (OtherActor :type "Actor Object Reference") (OtherComp :type "PrimitiveComponent Object Reference") (OtherBodyIndex :type Integer))
  ;[1 1 1] Attacking the Player
  ;;[1 1 1] Detecting if the Enemy can see the player
  (cast `/Game/Blueprint/Player/BP_Player` OtherActor)
  (if (not (`self.IsDead`))
    (set `self.CanSee` false)
    (`BlackboardComponent.SetValueAsBool` (`/Game/Blueprint/Enemy/Controllers/BP_EnemyController.Blackboard Component` (`self.ControllerReference`)) "CanSee" false)))

(event `self.CanAttack.OnComponentBeginOverlap`
  (params (OverlappedComponent :type "PrimitiveComponent Object Reference") (OtherActor :type "Actor Object Reference") (OtherComp :type "PrimitiveComponent Object Reference") (OtherBodyIndex :type Integer) (bFromSweep :type Boolean) (SweepResult :type "HitResult Structure (by ref)"))
  ;[1 1 1] Attacking the Player
  ;;[1 1 1] Detecting if the Enemy can attack the player
  (cast `/Game/Blueprint/Player/BP_Player` OtherActor)
  (if (not (`self.IsDead`))
    (`BlackboardComponent.SetValueAsBool` (`/Game/Blueprint/Enemy/Controllers/BP_EnemyController.Blackboard Component` (`self.ControllerReference`)) "CanAttack" true)))

(event `self.CanAttack.OnComponentEndOverlap`
  (params (OverlappedComponent :type "PrimitiveComponent Object Reference") (OtherActor :type "Actor Object Reference") (OtherComp :type "PrimitiveComponent Object Reference") (OtherBodyIndex :type Integer))
  ;[1 1 1] Attacking the Player
  ;;[1 1 1] Detecting if the Enemy can attack the player
  (cast `/Game/Blueprint/Player/BP_Player` OtherActor)
  (if (not (`self.IsDead`))
    (`BlackboardComponent.SetValueAsBool` (`/Game/Blueprint/Enemy/Controllers/BP_EnemyController.Blackboard Component` (`self.ControllerReference`)) "CanAttack" false)))

(event `Attack`
  (bind _mesh (`self.Mesh`))
  ;[1 1 1] Attacking the Player
  ;;[1 1 1] The Attacking Event
  (`/Engine/EditorBlueprintResources/StandardMacros.DoOnce` false :!label _label
    (:`Completed`
      (if (not (`self.IsDead`))
        (set `self.IsAttacking` true)
        (`CharacterMovementComponent.SetMovementMode` (`self.CharacterMovement`) "MOVE_None" 0)
        (`SkeletalMeshComponent.PlayAnimation` _mesh "/Game/Animations/Enemy/Standing_Melee_Attack_Horizontal.Standing_Melee_Attack_Horizontal" false)
        (`KismetSystemLibrary.Delay` 2.37)
        (if (not (`self.IsDead`))
          (`SkeletalMeshComponent.SetAnimationMode` _mesh "AnimationBlueprint")
          (`CharacterMovementComponent.SetMovementMode` (`self.CharacterMovement`) "MOVE_Walking" 0)
          (`self.ResetAttackAnimation`)
          (`self.ResetAttack`)
          (set `self.IsAttacking` false))))))

(event `ResetAttackAnimation`
  ;[1 1 1] Attacking the Player
  ;;[1 1 1] The Attacking Event
  (goto _label :!via `Reset`))

(event `InterruptAttack`
  ;[1 1 1] Attacking the Player
  ;;[1 1 1] Interrupt the Attacking
  (if (`self.IsAttacking`)
    (`SkeletalMeshComponent.Stop` (`self.Mesh`))))

(event `self.Weapon.OnComponentBeginOverlap`
  (params (OverlappedComponent :type "PrimitiveComponent Object Reference") (OtherActor :type "Actor Object Reference") (OtherComp :type "PrimitiveComponent Object Reference") (OtherBodyIndex :type Integer) (bFromSweep :type Boolean) (SweepResult :type "HitResult Structure (by ref)"))
  ;[1 1 1] Dealing Damage to the Player
  (bind _asbp_player (cast `/Game/Blueprint/Player/BP_Player` OtherActor))
  (`/Engine/EditorBlueprintResources/StandardMacros.DoOnce` false :!label _label_2
    (:`Completed`
      (`GameplayStatics.ApplyDamage` _asbp_player 10.0)
      (if (<= (- (`KismetMathLibrary.Conv_IntToDouble` (`/Game/Blueprint/BP_StatsComponent.Health` (`/Game/Blueprint/Player/BP_Player.BP_StatsComponent` _asbp_player))) (`.Damage_2_A53C99C447DED3E999EB858548ECFC36` (break `/Game/Structure/Struct_WeaponInfo` (`self.WeaponInfo`)))) 0.0)
        (set `self.IsPlayerDead` true)
        (`KismetSystemLibrary.PrintString` "Hello")
        (else
          (set `self.IsPlayerDead` false))))))

(event `ResetAttack`
  ;[1 1 1] Dealing Damage to the Player
  (goto _label_2 :!via `Reset`))

(event `Test`
  (params (Duration :type "Float (double-precision)")))

(fn `UserConstructionScript`
  ;[1 1 1] Getting the Correct Weapon Information
  (bind _weaponinfo (`/Game/Blueprint/BP_StatsComponent.WeaponDamage` (`self.BP_StatsComponent`) (`self.Weapon`)))
  (set `self.WeaponInfo` _weaponinfo))