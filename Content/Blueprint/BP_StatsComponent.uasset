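; BP_StatsComponent is a stats component that tracks Health through damage and healing functions.
; TakeDamage subtracts Health from Amount, reversed from the usual order, so Health drops to zero and Death runs whenever Amount is at most Health.
; Otherwise, the difference becomes the new Health.
; GiveHealth adds Amount clamped between zero and MaxHealth, and Death is an empty stub.
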(fn `Death`)

(fn `Give Health`
  (params (Amount :type Integer))
  (set `self.Health` (`KismetMathLibrary.Clamp` (+ Amount (`self.Health`)) 0 (`self.MaxHealth`))))

(fn `Take Damage`
  (params (Amount :type Integer))
  (bind _returnvalue (- Amount (`self.Health`)))
  (if (<= _returnvalue 0)
    (set `self.Health` 0)
    (`self.Death`)
    (else
      (set `self.Health` _returnvalue))))