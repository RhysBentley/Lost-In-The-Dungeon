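; Master inventory pickup item that the player collects or uses, with its mesh hovering and rotating via a randomly delayed timeline.
; Construction fills ItemInfo from the DT_Items row whose index matches ID when no valid item class is set.
; Collision overlap toggles input; Interaction stores weapons and consumables in BPInventoryComponent, while collectables call UseItem immediately.
; UseItem decrements or removes the inventory entry, then refreshes the inventory widget and player slots.
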(event `self.ReceiveBeginPlay`
  ;[0 0 0] Event Beginplay
  ;;[0 0 0] Getting Reference
  (bind _asbp_player (cast `/Game/Blueprint/Player/BP_Player` (`GameplayStatics.GetPlayerCharacter` 0)))
  (set `self.PlayerReference` _asbp_player)
  ;;[0 0 0] Rotate and Hover the Item
  (`KismetSystemLibrary.Delay` (`KismetMathLibrary.RandomFloatInRange` 0.2 1.0))
  (set `self.StartTransform` (`SceneComponent.K2_GetComponentToWorld` (`self.Mesh`)))
  (bind (_direction _alpha _rotation) (`Timeline|RotateItem`)
    (:`Update`
      (`SceneComponent.K2_SetWorldTransform` (`self.Mesh`) (`KismetMathLibrary.TLerp` (`self.StartTransform`) (`KismetMathLibrary.MakeTransform` (+ (.location (`self.StartTransform`)) (0.0 0.0 25.0)) (`KismetMathLibrary.MakeRotator` 0.0 0.0 (+ (.yaw (.rotation (`self.StartTransform`))) (.z _rotation)))) _alpha) false false))))

(event `self.Collision.OnComponentBeginOverlap`
  (params (OverlappedComponent :type "PrimitiveComponent Object Reference") (OtherActor :type "Actor Object Reference") (OtherComp :type "PrimitiveComponent Object Reference") (OtherBodyIndex :type Integer) (bFromSweep :type Boolean) (SweepResult :type "HitResult Structure (by ref)"))
  ;[0 0 0] Enabling Input when player is in range
  (cast `/Game/Blueprint/Player/BP_Player` OtherActor)
  (`self.EnableInput` (`GameplayStatics.GetPlayerController` 0)))

(event `self.Collision.OnComponentEndOverlap`
  (params (OverlappedComponent :type "PrimitiveComponent Object Reference") (OtherActor :type "Actor Object Reference") (OtherComp :type "PrimitiveComponent Object Reference") (OtherBodyIndex :type Integer))
  ;[0 0 0] Enabling Input when player is in range
  (cast `/Game/Blueprint/Player/BP_Player` OtherActor)
  (`self.DisableInput` (`GameplayStatics.GetPlayerController` 0)))

(event `InputAction|Interaction`
  (params (Key :type "Key Structure"))
  ;[0 0 0] Picking up the item
  (:`Pressed`
    (switch `/Game/Enumeration/Enum_ItemType` (`.ItemType_33_4B8B00E74F0795BAF69D4A96CD8FD2C7` (break `/Game/Structure/Struct_InventoryItem` (`self.ItemInfo`)))
      (:`NewEnumerator0`
        (`/Game/Blueprint/Inventory/BP_InventoryComponent.AddItem` (`/Game/Blueprint/Player/BP_Player.BP_InventoryComponent` (`self.PlayerReference`)) (`self.ItemInfo`) :!label _label)
        (`/Game/Widgets/Inventory/Widget_Inventory.UpdateInventorySlots` (`/Game/Widgets/Widget_HUD.Widget_Inventory` (`/Game/Blueprint/Player/BP_Player.HUDReference` (`self.PlayerReference`))))
        (`self.K2_DestroyActor`))
      (:`NewEnumerator1`
        (goto _label))
      (:`NewEnumerator2`
        (`self.UseItem`)
        (`self.K2_DestroyActor`)))))

(event `UseItem`
  (bind _inventory (`/Game/Blueprint/Inventory/BP_InventoryComponent.Inventory` (`/Game/Blueprint/Player/BP_Player.BP_InventoryComponent` (`self.PlayerReference`))))
  (bind _inventory_2 (`/Game/Blueprint/Inventory/BP_InventoryComponent.Inventory` (`/Game/Blueprint/Player/BP_Player.BP_InventoryComponent` (`self.PlayerReference`))))
  (bind _returnvalue (`KismetArrayLibrary.Array_Find` _inventory_2 (`self.ItemInfo`)))
  (bind _output (`|GetArrayItem` _inventory (`KismetArrayLibrary.Array_Find` _inventory (`self.ItemInfo`))))
  ;[0 0 0] When the Use Button is pressed
  (if (<= (`.Quantity_25_CCABC0304EA3051D0B5A609EAA090952` (break `/Game/Structure/Struct_InventoryItem` (`self.ItemInfo`))) 1)
    (if (not (<= _returnvalue -1))
      (`KismetArrayLibrary.Array_RemoveItem` _inventory_2 (`|GetArrayItem` _inventory_2 _returnvalue))
      (`/Game/Widgets/Inventory/Widget_Inventory.UpdateInventorySlots` (`/Game/Widgets/Widget_HUD.Widget_Inventory` (`/Game/Blueprint/Player/BP_Player.HUDReference` (`self.PlayerReference`))) :!label _label_2)
      (`/Game/Blueprint/Player/BP_Player.SettingSlots` (`self.PlayerReference`) (`self.ItemInfo`)))
    (else
      (setmembers `/Game/Structure/Struct_InventoryItem` :`StructRef` _output :`Quantity` (- (`.Quantity_25_CCABC0304EA3051D0B5A609EAA090952` (break `/Game/Structure/Struct_InventoryItem` _output)) 1))
      (goto _label_2))))

(fn `UserConstructionScript`
  (if (not (`KismetSystemLibrary.IsValidClass` (`.BlueprintClass_12_A3BE8845484EA4E75981A09D99305B41` (break `/Game/Structure/Struct_InventoryItem` (`self.ItemInfo`)))))
    ;[0 0 0] Getting the correct info for the item from the ID
    (bind _outrownames (`DataTableFunctionLibrary.GetDataTableRowNames` "/Game/DataTable/DT_Items.DT_Items"))
    (for (_array_element _array_index) _outrownames
      (bind _returnvalue (`|GetDataTableRow` "/Game/DataTable/DT_Items.DT_Items" _array_element)
        (:`then`
          (if (== _array_index (`self.ID`))
            (set `self.ItemInfo` _returnvalue)))))
    ;[0 0 0] Setting the item info
    (`StaticMeshComponent.SetStaticMesh` (`self.Mesh`) (`.StaticMesh_8_0B6818A94C13B8EBCB6B1B892388F204` (break `/Game/Structure/Struct_InventoryItem` (`self.ItemInfo`))))))