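; BP_Item_Potion is an inventory item that heals the player when used.
; UseItem gives a fixed amount of health through the player's stats component, then refreshes the health bar on the HUD's player stats widget.
; It also swaps the player's particle component to the NS_Healing effect and activates it before calling the parent UseItem logic.
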(event `self.ReceiveBeginPlay`
  (`parent.ReceiveBeginPlay`))

(event `self.UseItem`
  (bind _particle (`/Game/Blueprint/Player/BP_Player.Particle` (`self.PlayerReference`)))
  (`/Game/Blueprint/BP_StatsComponent.Give Health` (`/Game/Blueprint/Player/BP_Player.BP_StatsComponent` (`self.PlayerReference`)) 20)
  (`/Game/Widgets/Widget_PlayerStats.UpdateHealthBar` (`/Game/Widgets/Widget_HUD.Widget_PlayerStats` (`/Game/Blueprint/Player/BP_Player.HUDReference` (`self.PlayerReference`))))
  (`NiagaraComponent.SetAsset` _particle "/Game/Particle/NS_Healing.NS_Healing")
  (`ActorComponent.Activate` _particle true)
  (`parent.UseItem`))

(fn `UserConstructionScript`
  (`parent.UserConstructionScript`))