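; BP_ItemMaster is a pickup item actor that the player collects into their inventory with the Interaction input.
; The construction script looks up the DT_Items row whose index matches ID, stores it as ItemInfo and sets the mesh from it.
; Overlapping Collision toggles input for the player.
; Interacting adds ItemInfo to the player's inventory component, refreshes the HUD inventory slots and destroys the actor.
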(event `self.ReceiveBeginPlay`
  ;[0 0 0] Getting Reference
  (bind _asbp_player (cast `/Game/Blueprint/Player/BP_Player` (`GameplayStatics.GetPlayerCharacter` 0)))
  (set `self.PlayerReference` _asbp_player))

(event `self.Collision.OnComponentBeginOverlap`
  (params (OverlappedComponent :type "PrimitiveComponent Object Reference") (OtherActor :type "Actor Object Reference") (OtherComp :type "PrimitiveComponent Object Reference") (OtherBodyIndex :type Integer) (bFromSweep :type Boolean) (SweepResult :type "HitResult Structure (by ref)"))
  ;[0 0 0] Enabling Input when player is in range
  (cast `/Game/Blueprint/Player/BP_Player` OtherActor)
  (`self.EnableInput` (`GameplayStatics.GetPlayerController` 0)))

(event `self.Collision.OnComponentEndOverlap`
  (params (OverlappedComponent :type "PrimitiveComponent Object Reference") (OtherActor :type "Actor Object Reference") (OtherComp :type "PrimitiveComponent Object Reference") (OtherBodyIndex :type Integer))
  ;[0 0 0] Enabling Input when player is in range
  (cast `/Game/Blueprint/Player/BP_Player` OtherActor)
  (`self.DisableInput` (`GameplayStatics.GetPlayerController` 0)))

(event `InputAction|Interaction`
  (params (Key :type "Key Structure"))
  ;[0 0 0] Picking up the item
  (:`Pressed`
    (`/Game/Blueprint/Inventory/BP_InventoryComponent.AddItem` (`/Game/Blueprint/Player/BP_Player.BP_InventoryComponent` (`self.PlayerReference`)) (`self.ItemInfo`))
    (`/Game/Widgets/Widget_Inventory.UpdateInventorySlots` (`/Game/Widgets/Widget_HUD.Widget_Inventory` (`/Game/Blueprint/Player/BP_Player.HUDReference` (`self.PlayerReference`))))
    (`self.K2_DestroyActor`)))

(fn `UserConstructionScript`
  ;[0 0 0] Getting the correct info for the item from the ID
  (bind _outrownames (`DataTableFunctionLibrary.GetDataTableRowNames` "/Game/DataTable/DT_Items.DT_Items"))
  (for (_array_element _array_index) _outrownames
    (bind _returnvalue (`|GetDataTableRow` "/Game/DataTable/DT_Items.DT_Items" _array_element)
      (:`then`
        (if (== _array_index (`self.ID`))
          (set `self.ItemInfo` _returnvalue)))))
  ;[0 0 0] Setting the item info
  (`StaticMeshComponent.SetStaticMesh` (`self.Mesh`) (`.StaticMesh_8_0B6818A94C13B8EBCB6B1B892388F204` (break `/Game/Structure/Struct_InventoryItem` (`self.ItemInfo`)))))