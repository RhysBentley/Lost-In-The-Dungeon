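; BP_Item_Coin is a coin item Blueprint that adds to the player's money when used.
; UseItem increments the Coin count on PlayerReference, then calls UpdateMoney on the HUD's money widget to refresh it.
; BeginPlay and the construction script only call their parent versions.
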(event `self.ReceiveBeginPlay`
  (`parent.ReceiveBeginPlay`))

(event `self.UseItem`
  (`/Engine/EditorBlueprintResources/StandardMacros.IncrementInt` (`/Game/Blueprint/Player/BP_Player.Coin` (`self.PlayerReference`))
    (:`  `
      (`/Game/Widgets/Widget_Money.UpdateMoney` (`/Game/Widgets/Widget_HUD.Widget_Money` (`/Game/Blueprint/Player/BP_Player.HUDReference` (`self.PlayerReference`)))))))

(fn `UserConstructionScript`
  (`parent.UserConstructionScript`))