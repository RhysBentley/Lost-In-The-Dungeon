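; BP_Item_PaperMaster is a tutorial paper item, named as a master Blueprint, that shows readable text to the player.
; The Interaction input toggles Text through TutioralDialogue.ShowText, using IsHidden to track visibility.
; Ending an overlap with the Collision component hides the text and resets that flag, with no check on which actor left.
; BeginPlay caches the player as BP_Player, though these graphs never use that reference.
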(event `self.ReceiveBeginPlay`
  (bind _asbp_player (cast `/Game/Blueprint/Player/BP_Player` (`GameplayStatics.GetPlayerCharacter` 0)))
  (set `self.PlayerReference` _asbp_player))

(event `InputAction|Interaction`
  (params (Key :type "Key Structure"))
  (:`Pressed`
    (if (`self.IsHidden`)
      (`/Game/Blueprint/BP_TutioralDialogue.ShowText` (`self.TutioralDialogue`) (`self.Text`) false)
      (set `self.IsHidden` false)
      (else
        (`/Game/Blueprint/BP_TutioralDialogue.ShowText` (`self.TutioralDialogue`) (`self.Text`) true)
        (set `self.IsHidden` true)))))

(event `self.Collision.OnComponentEndOverlap`
  (params (OverlappedComponent :type "PrimitiveComponent Object Reference") (OtherActor :type "Actor Object Reference") (OtherComp :type "PrimitiveComponent Object Reference") (OtherBodyIndex :type Integer))
  (`/Game/Blueprint/BP_TutioralDialogue.ShowText` (`self.TutioralDialogue`) (`self.Text`) true)
  (set `self.IsHidden` true))

(fn `UserConstructionScript`)