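; Inventory component that stores item structs and handles adding, stacking and dropping items.
; On BeginPlay it seeds the inventory with DT_Items rows whose row index appears in IDToAdd.
; AddItem increments the quantity of an entry with a matching ID, otherwise appends the item.
; DropItem decrements the stack or removes its last entry, spawning a BP_Item__Master with that ID at the given transform.
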(event `self.ReceiveBeginPlay`
  ;[0 0 0] Add items that have been set to be in the inventory from the start
  (bind _outrownames (`DataTableFunctionLibrary.GetDataTableRowNames` "/Game/DataTable/DT_Items.DT_Items"))
  (for (_array_element _array_index) _outrownames
    (bind _returnvalue (`|GetDataTableRow` "/Game/DataTable/DT_Items.DT_Items" _array_element)
      (:`then`
        (if (`KismetArrayLibrary.Array_Contains` (`self.IDToAdd`) _array_index)
          (`KismetArrayLibrary.Array_Add` (`self.Inventory`) _returnvalue))))))

(event `AddItem`
  (params (ItemInfo :type "/Game/Structure/Struct_InventoryItem Structure"))
  (bind _inventory (`self.Inventory`))
  (bind _output (`|GetArrayItem` _inventory (`KismetArrayLibrary.Array_Find` _inventory (`self.Temp_ItemInfo`))))
  ;[0 0 0] Adds the item to the inventory
  (for _array_element (`self.Inventory`) :!label _label
    (if (== (`.ID_27_F5629E724BE2FB4174B3D4B082B40F19` (break `/Game/Structure/Struct_InventoryItem` _array_element)) (`.ID_27_F5629E724BE2FB4174B3D4B082B40F19` (break `/Game/Structure/Struct_InventoryItem` ItemInfo))) :!pinned true
      (set `self.HasItem?` true)
      (set `self.Temp_ItemInfo` _array_element)
      (`self.AddItemBreak`)
      (else
        (set `self.HasItem?` false))))
  (if (`self.HasItem?`)
    (setmembers `/Game/Structure/Struct_InventoryItem` :`StructRef` _output :`Quantity` (+ (`.Quantity_25_CCABC0304EA3051D0B5A609EAA090952` (break `/Game/Structure/Struct_InventoryItem` _output)) 1)) ; Adds to Item in Inventory
    (set `self.HasItem?` false)
    (else
      (`KismetArrayLibrary.Array_Add` (`self.Inventory`) ItemInfo :!pinned true) ; Simply Adds Item to Inventory
    )))

(event `AddItemBreak`
  ;[0 0 0] Adds the item to the inventory
  (goto _label :!via `Break`))

(event `DropItem`
  (params (ItemInfo :type "/Game/Structure/Struct_InventoryItem Structure") (SpawnTransform :type "Transform Structure"))
  (bind _inventory (`self.Inventory`))
  (bind _inventory_2 (`self.Inventory`))
  (bind _output (`|GetArrayItem` _inventory (`KismetArrayLibrary.Array_Find` _inventory ItemInfo)))
  ;[0 0 0] Drops the select item at the location given
  (if (<= (`.Quantity_25_CCABC0304EA3051D0B5A609EAA090952` (break `/Game/Structure/Struct_InventoryItem` ItemInfo)) 1)
    (`|SpawnActorFromClass` "/Game/Blueprint/Inventory/Items/BP_Item__Master.BP_Item__Master_C" SpawnTransform "Undefined" "OverrideRootScale" null (struct) (`.ID_27_F5629E724BE2FB4174B3D4B082B40F19` (break `/Game/Structure/Struct_InventoryItem` (`|GetArrayItem` _inventory_2 (`KismetArrayLibrary.Array_Find` _inventory_2 ItemInfo)))) null)
    (`KismetArrayLibrary.Array_RemoveItem` (`self.Inventory`) ItemInfo)
    (else
      (bind _structout (setmembers `/Game/Structure/Struct_InventoryItem` :`StructRef` _output :`Quantity` (- (`.Quantity_25_CCABC0304EA3051D0B5A609EAA090952` (break `/Game/Structure/Struct_InventoryItem` _output)) 1)))
      (`|SpawnActorFromClass` "/Game/Blueprint/Inventory/Items/BP_Item__Master.BP_Item__Master_C" SpawnTransform "Undefined" "OverrideRootScale" null (struct) (`.ID_27_F5629E724BE2FB4174B3D4B082B40F19` (break `/Game/Structure/Struct_InventoryItem` _structout)) null))))

(fn `BeforeRemoveItem`)